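; BP_Floor is an actor Blueprint that builds a rectangular grid of a chosen actor class, likely serving as tiled flooring.
; The construction script calls Generate, which adds a child actor component for each cell when ActorToSpawn is valid.
; A single flattened loop converts each index into X and Y offsets using division and modulo, scaled by Spacing.
; The event graph holds no active logic.
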(event EventBeginPlay)

(event Collision|EventActorBeginOverlap
  (params (OtherActor :type Actor%20Object%20Reference)))

(event EventTick
  (params (DeltaSeconds :type Float%20%28single-precision%29)))

(fn ConstructionScript
  (CallFunction|Generate))

(fn Generate
  (if (Utilities|IsValidClass (Variables|Default|GetActorToSpawn))
    (for _index (range 0 (- (* (Variables|Default|GetMaxX) (Variables|Default|GetMaxY)) 1))
      (bind _returnvalue (AddComponent|AddChildActorComponent false (Math|Transform|MakeTransform (Math|Vector|MakeVector (* (/ _index (Variables|Default|GetMaxY)) (Variables|Default|GetSpacing)) (* (Math|Integer|%(Integer) _index (Variables|Default|GetMaxY)) (Variables|Default|GetSpacing)) 0.0) "0, 0, 0" "1,1,1")))
      (ChildActorComponent|SetChildActorClass _returnvalue (Variables|Default|GetActorToSpawn)))))
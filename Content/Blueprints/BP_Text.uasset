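; BP_Text is an actor that shows configurable text in the world through a widget component.
; On BeginPlay it creates a WB_Text widget with its Text variable and assigns it to the component.
; It then sets the component's relative yaw toward the player pawn's location, computed once at start rather than updated every frame.
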(event EventBeginPlay
  (bind _returnvalue (UserInterface|CreateWidget "/Game/UI/WB_Text.WB_Text_C" 0 (Variables|Default|GetText)))
  (UserInterface|SetWidget (Variables|Default|GetWidget) _returnvalue)
  (Transformation|SetRelativeRotation (Variables|Default|GetWidget) (Math|Rotator|MakeRotator 0.0 0.0 (.yaw (Math|Rotator|FindLookatRotation (Transformation|GetActorLocation) (Transformation|GetActorLocation (Pawn|GetControlledPawn (Game|GetPlayerController 0)))))) false false))

(fn ConstructionScript)